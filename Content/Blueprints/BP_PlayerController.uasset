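; Player controller that drives a text-based branching scenario from the DT_FinalScenarioMASTERfinal data table.
; BeginPlay unpacks the rows into parallel arrays.
; Left-click release advances the text and shows choice buttons on BP_Userinterface, or on End commands records the unlocked ending in the GameInstance and displays it.
; CheckEvent hand-parses each row's comma-separated event string character by character into type, single-character code and position, passing each to CallSpawnNow.
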(event EventBeginPlay
  (Input|EnableInput self)
  (bind _outrownames (DataTable|GetDataTableRowNames "/Game/Scenario/DT_FinalScenarioMASTERfinal.DT_FinalScenarioMASTERfinal"))
  (for (_array_element _array_index) _outrownames
    (bind _returnvalue (Utilities|GetDataTableRow "/Game/Scenario/DT_FinalScenarioMASTERfinal.DT_FinalScenarioMASTERfinal" _array_element)
      (:then
        (Utilities|Array|SetArrayElem (Variables|Default|GetDispTextArray) _array_index (Utilities|Array|Get(acopy) (.text _returnvalue)) true)
        (Utilities|Array|SetArrayElem (Variables|Default|GetOutRowEventArray) _array_index (Utilities|Array|Get(acopy) (.event _returnvalue)) true)
        (Utilities|Array|SetArrayElem (Variables|Default|GetWhoIDArray) _array_index (Utilities|Array|Get(acopy) (.who_id _returnvalue)) true)
        (Utilities|Array|SetArrayElem (Variables|Default|GetOutRowBranch1Array) _array_index (Utilities|Array|Get(acopy) (.branch1 _returnvalue)) true)
        (Utilities|Array|SetArrayElem (Variables|Default|GetOutRowB1Array) _array_index (Utilities|Array|Get(acopy) (.b1 _returnvalue)) true)
        (Utilities|Array|SetArrayElem (Variables|Default|GetOutRowBranch2Array) _array_index (Utilities|Array|Get(acopy) (.branch2 _returnvalue)) true)
        (Utilities|Array|SetArrayElem (Variables|Default|GetOutRowB2Array) _array_index (Utilities|Array|Get(acopy) (.b2 _returnvalue)) true)
        (Utilities|Array|SetArrayElem (Variables|Default|GetOutRowBranch3Array) _array_index (Utilities|Array|Get(acopy) (.branch3 _returnvalue)) true)
        (Utilities|Array|SetArrayElem (Variables|Default|GetOutRowB3Array) _array_index (Utilities|Array|Get(acopy) (.b3 _returnvalue)) true)
        (Utilities|Array|SetArrayElem (Variables|Default|GetOutRowBranch4Array) _array_index (Utilities|Array|Get(acopy) (.branch4 _returnvalue)) true)
        (Utilities|Array|SetArrayElem (Variables|Default|GetOutRowB4Array) _array_index (Utilities|Array|Get(acopy) (.b4 _returnvalue)) true)
        (Utilities|Array|SetArrayElem (Variables|Default|GetCommandArray) _array_index (Utilities|Array|Get(acopy) (.command _returnvalue)) true)
        (if (or (Utilities|Enum|Equal(Enum) (Utilities|Array|Get(acopy) (Variables|Default|GetCommandReference) (Variables|Default|GetCommandReferenceIndex)) (Utilities|Array|Get(acopy) (.command _returnvalue))) false)
          (Utilities|Array|Add (Variables|Default|GetCommandIndex) (+ _array_index 1))
          (Variables|Default|SetCommandReferenceIndex (+ (Variables|Default|GetCommandReferenceIndex) 1)))
        (Utilities|Array|SetArrayElem (Variables|Default|GetImageID) (Utilities|Array|Get(acopy) (.imageid _returnvalue)) _array_index true)))))

(event Input|MouseEvents|LeftMouseButton
  (params (Key :type Key%20Structure :default "AnyKey"))
  (bind _gameinstance (Variables|Default|GetGameInstance))
  (bind _gameinstance_2 (Variables|Default|GetGameInstance))
  (bind _gameinstance_3 (Variables|Default|GetGameInstance))
  (bind _gameinstance_4 (Variables|Default|GetGameInstance))
  (bind _gameinstance_5 (Variables|Default|GetGameInstance))
  (:Released
    (bind _end (CallFunction|CheckEnd))
    (if _end
      (switch string (Utilities|Array|Get(acopy) (Variables|Default|GetCommandArray) (Variables|Default|GetMessageIndex))
        (:End0
          (Utilities|Array|SetArrayElem (Variables|/Game/Blueprints/BP_GameInstance.BP_GameInstance_C|GetCanWatchEnding _gameinstance) 0 true true)
          (Variables|/Game/Blueprints/BP_GameInstance.BP_GameInstance_C|SetClearEndingNumberBuf _gameinstance 0))
        (:End1
          (Utilities|Array|SetArrayElem (Variables|/Game/Blueprints/BP_GameInstance.BP_GameInstance_C|GetCanWatchEnding _gameinstance_2) 1 true true)
          (Variables|/Game/Blueprints/BP_GameInstance.BP_GameInstance_C|SetClearEndingNumberBuf _gameinstance_2 1))
        (:End2
          (Utilities|Array|SetArrayElem (Variables|/Game/Blueprints/BP_GameInstance.BP_GameInstance_C|GetCanWatchEnding _gameinstance_3) 2 true true)
          (Variables|/Game/Blueprints/BP_GameInstance.BP_GameInstance_C|SetClearEndingNumberBuf _gameinstance_3 2))
        (:End3
          (Utilities|Array|SetArrayElem (Variables|/Game/Blueprints/BP_GameInstance.BP_GameInstance_C|GetCanWatchEnding _gameinstance_4) 3 true true)
          (Variables|/Game/Blueprints/BP_GameInstance.BP_GameInstance_C|SetClearEndingNumberBuf _gameinstance_4 3))
        (:End4
          (Utilities|Array|SetArrayElem (Variables|/Game/Blueprints/BP_GameInstance.BP_GameInstance_C|GetCanWatchEnding _gameinstance_5) 4 true true)
          (Variables|/Game/Blueprints/BP_GameInstance.BP_GameInstance_C|SetClearEndingNumberBuf _gameinstance_5 4)))
      (bind _foundwidgets (Widget|GetAllWidgetsOfClass "/Game/Blueprints/UI/BP_Userinterface.BP_Userinterface_C" true))
      (Default|CanSeeTitleButton (Utilities|Array|Get(acopy) _foundwidgets))
      (Default|CanNotReturnButton (Utilities|Array|Get(acopy) _foundwidgets))
      (Default|EndingText (Utilities|Array|Get(acopy) _foundwidgets) (Variables|/Game/Blueprints/BP_GameInstance.BP_GameInstance_C|GetClearEndingNumberBuf (Variables|Default|GetGameInstance)))
      (else
        (CallFunction|CheckEvent)
        (switch string (Utilities|Array|Get(acopy) (Variables|Default|GetOutRowBranch1Array) (Variables|Default|GetMessageIndex))
          (:
            (Variables|Default|SetMessageIndex (Math|Integer|Clamp(Integer) (|({2175806D-4D9D-9514-7DAE-CF8942FB3268}+1)) 0 (Utilities|Array|Length (Variables|Default|GetDispTextArray))))
            (if (Utilities|Enum|NotEqual(Enum) (Utilities|Array|Get(acopy) (Variables|Default|GetOutRowEventArray) (Variables|Default|GetMessageIndex)) "")
              (bind _foundwidgets_2 (Widget|GetAllWidgetsOfClass "/Game/Blueprints/UI/BP_Userinterface.BP_Userinterface_C" true))
              ;[1 1 1] 次のテキストセット
              (Default|NextText (Utilities|Array|Get(acopy) _foundwidgets_2))
              (switch string (Utilities|Array|Get(acopy) (Variables|Default|GetCommandArray) (Variables|Default|GetMessageIndex))
                (:
                  (CallFunction|ShowCommandMenu)))
              (else
                (bind _foundwidgets_3 (Widget|GetAllWidgetsOfClass "/Game/Blueprints/UI/BP_Userinterface.BP_Userinterface_C" true))
                ;[1 1 1] 次のテキストセット
                (Default|NextText (Utilities|Array|Get(acopy) _foundwidgets_3))
                (switch string (Utilities|Array|Get(acopy) (Variables|Default|GetCommandArray) (Variables|Default|GetMessageIndex))
                  (:
                    (CallFunction|ShowCommandMenu)))))))))))

(fn ConstructionScript
  (bind _asbp_game_instance (Utilities|Casting|CastToBP_GameInstance (Game|GetGameInstance)))
  (Variables|Default|SetGameInstance _asbp_game_instance))

(fn ShowCommandMenu
  (bind _messageindex (Variables|Default|GetMessageIndex))
  (bind _outrowbranch4array (Variables|Default|GetOutRowBranch4Array))
  (bind _item (Utilities|Array|Get(acopy) _outrowbranch4array _messageindex))
  (bind _foundwidgets (Widget|GetAllWidgetsOfClass "/Game/Blueprints/UI/BP_Userinterface.BP_Userinterface_C" true))
  (if (Utilities|Enum|NotEqual(Enum) (Utilities|Array|Get(acopy) (Variables|Default|GetOutRowBranch1Array) (Variables|Default|GetMessageIndex)) "")
    (Rendering|Components|TextRender|SetText (Variables|/Game/Blueprints/UI/BP_Userinterface.BP_Userinterface_C|GetSentakusi1 (Utilities|Array|Get(acopy) _foundwidgets)) (Utilities|Text|ToText(String) (Utilities|Array|Get(acopy) (Variables|Default|GetOutRowBranch1Array) _messageindex)))
    (Rendering|Components|TextRender|SetText (Variables|/Game/Blueprints/UI/BP_Userinterface.BP_Userinterface_C|GetSentakusi2 (Utilities|Array|Get(acopy) _foundwidgets)) (Utilities|Text|ToText(String) (Utilities|Array|Get(acopy) (Variables|Default|GetOutRowBranch2Array) _messageindex)))
    (Rendering|Components|TextRender|SetText (Variables|/Game/Blueprints/UI/BP_Userinterface.BP_Userinterface_C|GetSentakusi3 (Utilities|Array|Get(acopy) _foundwidgets)) (Utilities|Text|ToText(String) (Utilities|Array|Get(acopy) (Variables|Default|GetOutRowBranch3Array) _messageindex)))
    (Rendering|Components|TextRender|SetText (Variables|/Game/Blueprints/UI/BP_Userinterface.BP_Userinterface_C|GetSentakusi4 (Utilities|Array|Get(acopy) _foundwidgets)) (Utilities|Text|ToText(String) _item))
    ;[1 1 1] 選択肢表示
    (Widget|SetVisibility (Variables|/Game/Blueprints/UI/BP_Userinterface.BP_Userinterface_C|GetSentakusi1B (Utilities|Array|Get(acopy) _foundwidgets)) "Visible")
    (Widget|SetVisibility (Variables|/Game/Blueprints/UI/BP_Userinterface.BP_Userinterface_C|GetSentakusi2B (Utilities|Array|Get(acopy) _foundwidgets)) "Visible")
    (Widget|SetVisibility (Variables|/Game/Blueprints/UI/BP_Userinterface.BP_Userinterface_C|GetSentakusi3B (Utilities|Array|Get(acopy) _foundwidgets)) "Visible")
    (if (not (Utilities|Enum|Equal(Enum) _item ""))
      (Widget|SetVisibility (Variables|/Game/Blueprints/UI/BP_Userinterface.BP_Userinterface_C|GetSentakusi4B (Utilities|Array|Get(acopy) _foundwidgets)) "Visible"))))

(fn CheckEnd
  (bind _messageindex (Variables|Default|GetMessageIndex))
  (bind _commandarray (Variables|Default|GetCommandArray))
  (bind _item (Utilities|Array|Get(acopy) _commandarray _messageindex))
  (return (Math|Boolean|ORBoolean (Utilities|Enum|Equal(Enum) _item "End0") (Utilities|Enum|Equal(Enum) _item "End1") (Utilities|Enum|Equal(Enum) _item "End2") (Utilities|Enum|Equal(Enum) _item "End3") (Utilities|Enum|Equal(Enum) _item "End4"))))

(fn CheckEvent
  (bind _outroweventarray (Variables|Default|GetOutRowEventArray))
  (bind _messageindex (Variables|Default|GetMessageIndex))
  (bind _order (Variables|Default|GetOrder))
  (bind _outroweventarray_2 (Variables|Default|GetOutRowEventArray))
  (bind _messageindex_2 (Variables|Default|GetMessageIndex))
  (bind _item (Utilities|Array|Get(acopy) _outroweventarray_2 _messageindex_2))
  (bind _item_2 (Utilities|Array|Get(acopy) _outroweventarray _messageindex))
  (bind _returnvalue (Utilities|String|GetCharacterArrayfromString _item_2))
  (bind _returnvalue_2 (Utilities|String|GetCharacterArrayfromString _item))
  (bind _returnvalue_3 (Utilities|Array|LastIndex _returnvalue_2))
  (bind _returnvalue_4 (Utilities|Array|LastIndex _returnvalue))
  (for _index (range (Variables|Default|GetloopIndex) (Utilities|Array|LastIndex _order))
    (if (!= (Variables|Default|GetConmaPos) 0)
      (if (Variables|Default|GetloopFLAG)
        ;[1 1 1] 2週目からこちら
        ;;[1 1 1] 中ループ第1 space探査
        (bind _index_2 (Utilities|FlowControl|ForLoopwithBreak (+ (Variables|Default|GetConmaPos) 1) (Utilities|Array|LastIndex _outroweventarray) :!label _label)
          (:LoopBody
            (if (Utilities|Enum|Equal(Enum) (Utilities|Array|Get(acopy) _returnvalue _index_2) " ")
              (bind _output_get (Variables|Default|SetspaceIndex _index_2))
              (goto _label Break)))
          (:Completed
            ;;[1 1 1] 中ループ第2 OrderType入れ
            (for _index_3 (range (+ (Variables|Default|GetConmaPos) 1) (- _output_get 1))
              (Variables|Default|SetOrderTypeTmp (Utilities|String|Append (Variables|Default|GetOrderTypeTmp) (Utilities|Array|Get(acopy) _returnvalue _index_3))))
            (Variables|Default|SetFirstConmaPos (Variables|Default|GetConmaPos))
            ;;[1 1 1] 中ループ第3 コンマ探し
            (bind _index_4 (Utilities|FlowControl|ForLoopwithBreak (+ (Variables|Default|GetConmaPos) 1) _returnvalue_4 :!label _label_2)
              (:LoopBody
                (if (Utilities|Enum|Equal(Enum) (Utilities|Array|Get(acopy) _returnvalue _index_4) ",")
                  (Variables|Default|SetConmaPos _index_4)
                  (goto _label_2 Break)))
              (:Completed
                (if (!= (Variables|Default|GetConmaPos) (Variables|Default|GetFirstConmaPos))
                  (for _index_5 (range (+ (Variables|Default|GetspaceIndex) 3) (- (Variables|Default|GetConmaPos) 1))
                    (Variables|Default|SetOrderPositionTmp (Utilities|String|Append (Variables|Default|GetOrderPositionTmp) (Utilities|Array|Get(acopy) _returnvalue _index_5))))
                  (bind _structout (Utilities|Struct|SetmembersinOrderstruct (Utilities|Array|Get(acopy) _order _index) (Variables|Default|GetOrderTypeTmp) (CallFunction|KanbanCodetoInt (Utilities|Array|Get(acopy) _returnvalue (+ (Variables|Default|GetspaceIndex) 1))) (Variables|Default|GetOrderPositionTmp)))
                  (Default|CallSpawnNow (.ordertype _structout) (.orderbp _structout) (.orderposition _structout))
                  (Variables|Default|SetOrderTypeTmp "")
                  (Variables|Default|SetOrderPositionTmp "")
                  (else
                    (for _index_6 (range (+ (Variables|Default|GetspaceIndex) 3) _returnvalue_4)
                      (Variables|Default|SetOrderPositionTmp (Utilities|String|Append (Variables|Default|GetOrderPositionTmp) (Utilities|Array|Get(acopy) _returnvalue _index_6))))
                    (bind _structout_2 (Utilities|Struct|SetmembersinOrderstruct (Utilities|Array|Get(acopy) _order _index) (Variables|Default|GetOrderTypeTmp) (CallFunction|KanbanCodetoInt (Utilities|Array|Get(acopy) _returnvalue (+ (Variables|Default|GetspaceIndex) 1))) (Variables|Default|GetOrderPositionTmp)))
                    (Default|CallSpawnNow (.ordertype _structout_2) (.orderbp _structout_2) (.orderposition _structout_2))
                    (Variables|Default|SetOrderTypeTmp "")
                    (Variables|Default|SetOrderPositionTmp "")
                    (Variables|Default|SetloopFLAG false))))))))
      (elif (Variables|Default|GetloopFLAG)
        ;[1 1 1] 中ループ第1 space探査
        (bind _index_7 (Utilities|FlowControl|ForLoopwithBreak 0 (Utilities|Array|LastIndex _outroweventarray_2) :!label _label_3)
          (:LoopBody
            (if (Utilities|Enum|Equal(Enum) (Utilities|Array|Get(acopy) _returnvalue_2 _index_7) " ")
              (bind _output_get_2 (Variables|Default|SetspaceIndex _index_7))
              (goto _label_3 Break)))
          (:Completed
            (for _index_8 (range 0 (- _output_get_2 1))
              (Variables|Default|SetOrderTypeTmp (Utilities|String|Append (Variables|Default|GetOrderTypeTmp) (Utilities|Array|Get(acopy) _returnvalue_2 _index_8))))
            ;[1 1 1] 中ループ第3 コンマ探し
            (bind _index_9 (Utilities|FlowControl|ForLoopwithBreak 0 _returnvalue_3 :!label _label_4)
              (:LoopBody
                (if (Utilities|Enum|Equal(Enum) (Utilities|Array|Get(acopy) _returnvalue_2 _index_9) ",")
                  (Variables|Default|SetConmaPos _index_9)
                  (goto _label_4 Break)))
              (:Completed
                (if (!= (Variables|Default|GetConmaPos) 0)
                  (for _index_10 (range (+ (Variables|Default|GetspaceIndex) 3) (- (Variables|Default|GetConmaPos) 1))
                    (Variables|Default|SetOrderPositionTmp (Utilities|String|Append (Variables|Default|GetOrderPositionTmp) (Utilities|Array|Get(acopy) _returnvalue_2 _index_10))))
                  (bind _structout_3 (Utilities|Struct|SetmembersinOrderstruct (Utilities|Array|Get(acopy) _order _index) (Variables|Default|GetOrderTypeTmp) (CallFunction|KanbanCodetoInt (Utilities|Array|Get(acopy) _returnvalue_2 (+ (Variables|Default|GetspaceIndex) 1))) (Variables|Default|GetOrderPositionTmp)))
                  (Default|CallSpawnNow (.ordertype _structout_3) (.orderbp _structout_3) (.orderposition _structout_3))
                  (Variables|Default|SetOrderTypeTmp "")
                  (Variables|Default|SetOrderPositionTmp "")
                  (else
                    (for _index_11 (range (+ (Variables|Default|GetspaceIndex) 3) _returnvalue_3)
                      (Variables|Default|SetOrderPositionTmp (Utilities|String|Append (Variables|Default|GetOrderPositionTmp) (Utilities|Array|Get(acopy) _returnvalue_2 _index_11))))
                    (bind _structout_4 (Utilities|Struct|SetmembersinOrderstruct (Utilities|Array|Get(acopy) _order _index) (Variables|Default|GetOrderTypeTmp) (CallFunction|KanbanCodetoInt (Utilities|Array|Get(acopy) _returnvalue_2 (+ (Variables|Default|GetspaceIndex) 1))) (Variables|Default|GetOrderPositionTmp)))
                    (Default|CallSpawnNow (.ordertype _structout_4) (.orderbp _structout_4) (.orderposition _structout_4))
                    (Variables|Default|SetloopFLAG false)
                    (Variables|Default|SetOrderTypeTmp "")
                    (Variables|Default|SetOrderPositionTmp ""))))))))))
  (Variables|Default|SetloopIndex 0)
  (Variables|Default|SetConmaPos 0)
  (Variables|Default|SetspaceIndex 0)
  (Variables|Default|SetFirstConmaPos 0)
  (Variables|Default|SetloopFLAG true)
  (Variables|Default|SetOrderTypeTmp "")
  (Variables|Default|SetOrderPositionTmp ""))

(fn KanbanCodetoInt
  (params (OrderNum :type String))
  (switch string OrderNum
    (:Default
      (return 100))
    (:0
      (return 0))
    (:1
      (return 1))
    (:2
      (return 2))
    (:3
      (return 3))
    (:4
      (return 4))
    (:5
      (return 5))
    (:6
      (return 6))
    (:7
      (return 7))
    (:8
      (return 8))
    (:9
      (return 9))
    (:A
      (return 10))
    (:B
      (return 11))
    (:C
      (return 12))
    (:D
      (return 13))
    (:E
      (return 14))
    (:F
      (return 15))
    (:G
      (return 16))
    (:H
      (return 17))
    (:I
      (return 18))
    (:J
      (return 19))
    (:K
      (return 20))))